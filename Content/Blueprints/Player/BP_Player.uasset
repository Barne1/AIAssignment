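; Player Blueprint that serves as an interactive debug tool for A* pathfinding on a tile grid.
; OnConfirm snaps the mouse position to a tile, clearing it if already start or end, otherwise filling the first empty endpoint.
; Once both are set, AStarComponent computes the path; clearing an endpoint leaves the previous result intact.
; Tick draws debug spheres for endpoints, cursor and intermediate path tiles, or prints a no-path warning.
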(event `self.ReceiveTick`
  (params (DeltaSeconds :type "Float (single-precision)"))
  (bind (_outworldmouselocation _returnvalue) (`self.GetMouseLocationOnGrid`))
  (bind _xypath (`self.XYPath`))
  (bind (_startpos_x _startpos_y) (break `IntPoint` (`self.StartPos`)))
  (bind (_endpos_x _endpos_y) (break `IntPoint` (`self.EndPos`)))
  (`|ExecutionSequence`
    (:`then_0`
      (`|ExecutionSequence`
        (:`then_0`
          (if (!= (`self.StartPos`) (make `IntPoint` -1 -1))
            (`KismetSystemLibrary.DrawDebugSphere` (`FGGridActor.GetWorldLocationFromXY` (`self.CurrentGridActor`) _startpos_x _startpos_y) 100.0 12 (struct :`R` 0.040045 :`G` 1.0 :`A` 1.0))))
        (:`then_1`
          (if (!= (`self.EndPos`) (make `IntPoint` -1 -1))
            (`KismetSystemLibrary.DrawDebugSphere` (`FGGridActor.GetWorldLocationFromXY` (`self.CurrentGridActor`) _endpos_x _endpos_y) 100.0 12 (struct :`R` 0.097319 :`B` 1.0 :`A` 1.0))))))
    (:`then_1`
      (if _returnvalue
        (`KismetSystemLibrary.DrawDebugSphere` _outworldmouselocation)))
    (:`then_2`
      (if (`self.PathFound`)
        (for (_array_element _array_index) _xypath
          (if (and (!= (- (`KismetArrayLibrary.Array_Length` _xypath) 1) _array_index) (!= _array_index 0))
            (`KismetSystemLibrary.DrawDebugSphere` (`FGGridActor.GetWorldLocationFromXY` (`self.CurrentGridActor`) (break `IntPoint` _array_element) (`.Y` (break `IntPoint` _array_element))) 100.0 12 (struct :`R` 1.0 :`G` 0.874285 :`A` 1.0))))
        (else
          (`KismetSystemLibrary.PrintString` "NO PATH" true false (struct :`R` 1.0 :`G` 0.010052 :`A` 1.0) 0.0))))))

(event `self.BP_OnConfirm`
  (bind (_outworldmouselocation _returnvalue) (`self.GetMouseLocationOnGrid`))
  (bind _currentgridactor (`self.CurrentGridActor`))
  (bind (_outtileworldlocation _returnvalue_2) (`FGGridActor.TransformWorldLocationToTileLocation` _currentgridactor _outworldmouselocation))
  (bind (_tilex _tiley) (`FGGridActor.GetXYFromWorldLocation` _currentgridactor _outtileworldlocation))
  (if (`.ReturnValue` (`self.GetMouseLocationOnGrid`))
    (`/Engine/EditorBlueprintResources/StandardMacros.IsValid` (`self.CurrentGridActor`)
      (:`Is Valid`
        (if _returnvalue
          (if _returnvalue_2
            (set `self.Clicked` (make `IntPoint` _tilex _tiley))
            (if (`KismetMathLibrary.Equal_IntPointIntPoint` (`self.StartPos`) (`self.Clicked`))
              (set `self.StartPos` (make `IntPoint` -1 -1))
              (elif (`KismetMathLibrary.Equal_IntPointIntPoint` (`self.Clicked`) (`self.EndPos`))
                (set `self.EndPos` (make `IntPoint` -1 -1))
                (elif (`KismetMathLibrary.Equal_IntPointIntPoint` (`self.StartPos`) (make `IntPoint` -1 -1))
                  (set `self.StartPos` (`self.Clicked`))
                  (if (and (!= (`self.EndPos`) (make `IntPoint` -1 -1)) (!= (`self.StartPos`) (make `IntPoint` -1 -1))) :!label _label
                    (bind (_outpath _returnvalue_3) (`FGAStarComponent.FindPathXY` (`self.AStarComponent`) (`self.CurrentGridActor`) (`self.StartPos`) (`self.EndPos`)))
                    (set `self.PathFound` _returnvalue_3)
                    (set `self.XYPath` _outpath)
                    (else
                      (`KismetSystemLibrary.PrintString` "CONDITION NOT MET" true true (struct :`R` 1.0 :`B` 0.335279 :`A` 1.0) 5.0)))
                  (elif (`KismetMathLibrary.Equal_IntPointIntPoint` (`self.EndPos`) (make `IntPoint` -1 -1))
                    (set `self.EndPos` (`self.Clicked`))
                    (goto _label)))))))))))

(fn `UserConstructionScript`)